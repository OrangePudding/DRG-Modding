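; Driller loot pod that delivers a gold-filled loot bug and bursts it into resources when dropped to terrain.
; It spawns an ENE_LootBug as the pod's alternate actor, caches it and freezes its movement.
; On landing it kills the bug and starts a fast looping timer that flings Red Sugar chunks upward in a random cone.
; A counter caps the chunks, though the timer is never cleared.
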(event Collision|EventActorBeginOverlap
  (params (OtherActor :type Actor%20Object%20Reference)))

(event EventTick
  (params (DeltaSeconds :type Float%20%28single-precision%29)))

(event EventBeginPlay
  (|CallParentFunction))

(fn ConstructionScript)

(fn OnDroppedtoTerrain
  (Class|HealthComponentBase|Kill (Variables|/Script/FSD.CaveWorm|GetHealth (Variables|Default|GetLoot)))
  (bind _returnvalue (Utilities|Time|SetTimerbyFunctionName 0 "SpawnChunk" 0.06 true))
  (Variables|Default|SetSpawnChunks _returnvalue))

(fn AlternateActorSpawnedFunc
  (params (Actor :type Actor%20Object%20Reference))
  (bind _asene_loot_bug (Utilities|Casting|CastToENE_LootBug Actor))
  (bind _output_get (Variables|Default|SetLoot _asene_loot_bug))
  (Variables|/Script/FSD.DeepPathfinderMovement|SetMaxPawnSpeed (Variables|/Script/FSD.DeepPathfinderCharacter|GetPathfinderMovement _output_get) 0.0)
  (Class|DeepPathfinderMovement|PauseMovement (Variables|/Script/FSD.DeepPathfinderCharacter|GetPathfinderMovement _output_get) 999.0))

(fn SpawnAlternateActor
  (bind _returnvalue (Game|SpawnActorfromClass "/Game/Critters/Lootbug/ENE_LootBug.ENE_LootBug_C" (Math|Transform|MakeTransform "0, 0, 0") "AlwaysSpawn" 0 "(X=85.000000,Y=110.000000)" "(X=1.500000,Y=2.500000)" (Utilities|Array|MakeArray "/Game/GameElements/Resources/Veins/RES_VEIN_Gold.RES_VEIN_Gold") 0))
  (return _returnvalue))

(fn SpawnChunk
  (if (< (Variables|Default|GetSpawnCounter) (Variables|Default|GetMaxSpawnCount))
    (Class|CaveWorm|DropResource (Variables|Default|GetLoot) "/Game/GameElements/Resources/Carved/RedSugar/RES_CARVED_RedSugar.RES_CARVED_RedSugar" (Math|Random|RandomFloatinRange 0.6 1.2) (* (Class|KismetMathLibrary|RandomUnitVectorinEllipticalConeinDegrees "0, 0,1.000000" 6e+01 6e+01) 2e+04) "0, 0,50.000000")
    (Variables|Default|SetSpawnCounter (+ (Variables|Default|GetSpawnCounter) 1))))