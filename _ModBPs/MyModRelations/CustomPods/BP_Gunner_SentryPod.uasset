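; Gunner sentry drop pod that delivers a modified Minehead sentry leaving sticky flames where its shots land.
; It fills in parent pod hooks to spawn the sentry, deploy it on reaching terrain and play its undeploy on takeoff.
; On landing it overrides ammo, rotation speed and hitscan spread, and adds a flame spawner fed by hit events.
; The pod attempts takeoff once the sentry's ammo runs out.
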(event Collision|EventActorBeginOverlap
  (params (OtherActor :type Actor%20Object%20Reference)))

(event EventTick
  (params (DeltaSeconds :type Float%20%28single-precision%29)))

(event EventBeginPlay
  (|CallParentFunction))

(fn ConstructionScript)

(fn OnAmmoCountChanged
  (params (AmmoCount :type Integer) (Change :type Integer))
  (if (< AmmoCount 1)
    (CallFunction|TryTakeOff)))

(fn OnDroppedtoTerrain
  (bind _sentry (Variables|Default|GetSentry))
  (bind _hitscan (Variables|/Game/WeaponsNTools/SentryGun/SentryGun_MineHead/BP_Minehead_Sentry.BP_Minehead_Sentry_C|GetHitscan _sentry))
  (Default|Deploy _sentry)
  (EventDispatchers|BindEventtoOnAmmoCountChanged _sentry (EventDispatchers|CreateEvent :!event OnAmmoCountChanged))
  (Utilities|FlowControl|Sequence
    (:then_0
      (Variables|/Script/FSD.SentryGun|SetMaxAmmoCount _sentry 200))
    (:then_1
      (Variables|/Script/FSD.SentryGun|SetAmmoCount _sentry 150)
      (Variables|/Script/FSD.SentryGun|SetRotationSpeed _sentry 2.6))
    (:then_2
      (bind _returnvalue (AddComponent|AddStickyFlameSpawner _sentry))
      (Variables|Default|SetStickyFlameSpawner _returnvalue))
    (:then_3
      (Variables|/Script/FSD.HitscanBaseComponent|SetMaxSpread _hitscan 9.0)
      (Variables|/Script/FSD.HitscanBaseComponent|SetMaxVerticalSpread _hitscan 6.0)
      (Variables|/Script/FSD.HitscanBaseComponent|SetMaxHorizontalSpread _hitscan 6.0)
      (Variables|/Script/FSD.HitscanBaseComponent|SetMinSpread _hitscan 4.5))
    (:then_4
      (EventDispatchers|BindEventtoOnHit _hitscan (EventDispatchers|CreateEvent :!event OnTurretHit)))))

(fn AlternateActorSpawnedFunc
  (params (Actor :type Actor%20Object%20Reference))
  (bind _asbp_minehead_sentry (Utilities|Casting|CastToBP_Minehead_Sentry Actor))
  (Variables|Default|SetSentry _asbp_minehead_sentry))

(fn ExtraTakeOffFunc
  (Components|Timeline|PlayfromStart (Variables|/Game/WeaponsNTools/SentryGun/SentryGun_MineHead/BP_Minehead_Sentry.BP_Minehead_Sentry_C|GetUndeploy (Variables|Default|GetSentry))))

(fn SpawnAlternateActor
  (bind _returnvalue (Game|SpawnActorfromClass "/Game/WeaponsNTools/SentryGun/SentryGun_MineHead/BP_Minehead_Sentry.BP_Minehead_Sentry_C" (Math|Transform|MakeTransform "0, 0, 0") "AlwaysSpawn" 0 0))
  (return _returnvalue))

(fn OnTurretHit
  (params (Hit :type Hit%20Result%20Structure%20%28by%20ref%29) (alwaysPenetrate :type Boolean))
  (bind (_bblockinghit _binitialoverlap _time _distance _location _impactpoint _normal) (Collision|BreakHitResult Hit))
  (Class|StickyFlameSpawner|ServerSpawnStickyFlame (Variables|Default|GetStickyFlameSpawner) (Class|FSDConversionLibrary|VectortoNetQuantize _location) (Class|FSDConversionLibrary|VectortoNetQuantizeNormal _normal)))