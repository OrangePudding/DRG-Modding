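; Scout pod variant that carries and deploys an interactive floodlight in place of the parent pod's usual payload.
; It overrides parent hooks to spawn a BP_SpotLightInteractive, cache it as Light and enable movement replication on it.
; Dropping to terrain activates the light, and the extra take-off hook reverses the light's timeline from the end.
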(event Collision|EventActorBeginOverlap
  (params (OtherActor :type Actor%20Object%20Reference)))

(event EventTick
  (params (DeltaSeconds :type Float%20%28single-precision%29)))

(event EventBeginPlay
  (|CallParentFunction))

(fn ConstructionScript)

(fn OnDroppedtoTerrain
  (Default|Activate (Variables|Default|GetLight)))

(fn AlternateActorSpawnedFunc
  (params (Actor :type Actor%20Object%20Reference))
  (bind _asbp_spot_light_interactive (Utilities|Casting|CastToBP_SpotLightInteractive Actor))
  (bind _output_get (Variables|Default|SetLight _asbp_spot_light_interactive))
  (Class|Actor|SetReplicateMovement _output_get true))

(fn ExtraTakeOffFunc
  (Components|Timeline|ReversefromEnd (Variables|/Game/LevelElements/Minehead/BP_SpotLightInteractive.BP_SpotLightInteractive_C|GetTimeline_1 (Variables|Default|GetLight))))

(fn SpawnAlternateActor
  (bind _returnvalue (Game|SpawnActorfromClass "/Game/LevelElements/Minehead/BP_SpotLightInteractive.BP_SpotLightInteractive_C" (Math|Transform|MakeTransform "0, 0, 0") "AlwaysSpawn" 0 0))
  (return _returnvalue))