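; BP_Engineer_DetonatorPod is a custom Engineer drop pod that delivers an exploding Detonator and leaves radiation behind.
; It overrides the alternate-actor spawn to create a scaled-down ENE_Spider_ExploderTank, then caches it and pauses its pathfinding.
; On reaching terrain it kills the Detonator through its health component and starts a short timer that spawns a BP_MiniNuke_RadiationCloud above the pod.
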(event Collision|EventActorBeginOverlap
  (params (OtherActor :type Actor%20Object%20Reference)))

(event EventTick
  (params (DeltaSeconds :type Float%20%28single-precision%29)))

(event EventBeginPlay
  (|CallParentFunction))

(fn ConstructionScript)

(fn OnDroppedtoTerrain
  (Class|HealthComponentBase|Kill (Variables|/Script/FSD.EnemyDeepPathfinderCharacter|GetHealthComponent (Variables|Default|GetDetonator)))
  (Utilities|Time|SetTimerbyFunctionName 0 "SpawnCloud" 2.5))

(fn AlternateActorSpawnedFunc
  (params (Actor :type Actor%20Object%20Reference))
  (bind _asene_spider_exploder_tank (Utilities|Casting|CastToENE_Spider_ExploderTank Actor))
  (bind _output_get (Variables|Default|SetDetonator _asene_spider_exploder_tank))
  (Class|DeepPathfinderMovement|PauseMovement (Variables|/Script/FSD.DeepPathfinderCharacter|GetPathfinderMovement _output_get) 999.0))

(fn SpawnAlternateActor
  (bind _returnvalue (Game|SpawnActorfromClass "/Game/Enemies/Spider/ExploderTank/ENE_Spider_ExploderTank.ENE_Spider_ExploderTank_C" (Math|Transform|MakeTransform "0, 0, 0" "0, 0, 0" "0.800000,0.800000,0.800000") "AlwaysSpawn" 0 0))
  (return _returnvalue))

(fn SpawnCloud
  (Game|SpawnActorfromClass "/Game/WeaponsNTools/GrenadeLauncher/BP_MiniNuke_RadiationCloud.BP_MiniNuke_RadiationCloud_C" (Math|Transform|MakeTransform (+ (Class|FSDConversionLibrary|ActortoWorldLocation self) "0, 0,220.000000") "0, 0, 0" "0.900000,0.900000,0.900000") "AlwaysSpawn" 0 0))