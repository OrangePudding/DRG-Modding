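; Base Blueprint for a custom grenade pod that launches a series of grenades once it is dropped to terrain.
; OnDroppedtoTerrain runs a custom ForLoopWithDelay macro, calling SpawnGrenade MaxNumber times at SpawnInterval spacing.
; Each GrenadeClass actor spawns at the pod's location plus MuzzleShift, facing a random direction in the upper hemisphere, with its movement velocity scaled by SpeedModifier.
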(event EventBeginPlay
  (|CallParentFunction) ; This node is disabled and will not be called.\nDrag off pins to build functionality.
)

(event Collision|EventActorBeginOverlap
  (params (OtherActor :type Actor%20Object%20Reference))
  (|CallParentFunction OtherActor) ; This node is disabled and will not be called.\nDrag off pins to build functionality.
)

(event EventTick
  (params (DeltaSeconds :type Float%20%28single-precision%29))
  (|CallParentFunction DeltaSeconds) ; This node is disabled and will not be called.\nDrag off pins to build functionality.
)

(event EventOnDroppedtoTerrain
  (Utilities|ForLoopwithDelay 0 (- (Variables|Default|GetMaxNumber) 1) (Variables|Default|GetSpawnInterval)
    (:LoopBody
      (CallFunction|SpawnGrenade))))

(fn ConstructionScript
  (|CallParentFunction))

(fn SpawnGrenade
  (bind _returnvalue (Game|SpawnActorfromClass (Variables|Default|GetGrenadeClass) (Math|Transform|MakeTransform (+ (Class|FSDConversionLibrary|ActortoWorldLocation self) (Variables|Default|GetMuzzleShift)) (Math|Conversions|RotationFromXVector (Math|Random|RandomUnitVectorinConeinDegrees "0, 0,1.000000" 9e+01))) "AlwaysSpawn" 0 0))
  (Variables|/Script/Engine.MovementComponent|SetVelocity (Variables|/Script/FSD.Grenade|GetMovement _returnvalue) (* (Variables|/Script/Engine.MovementComponent|GetVelocity (Variables|/Script/FSD.Grenade|GetMovement _returnvalue)) (Variables|Default|GetSpeedModifier))))