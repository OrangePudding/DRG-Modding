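; Base Blueprint for custom drop pods that reuse BP_HackingPod's drop and takeoff behavior to deliver a different actor.
; On BeginPlay it calls DropToTarget through a throwaway pod, then hides the new pod's base, monitors and range sphere and removes its dispenser.
; The actor from SpawnAlternateActor is attached to that base.
; Timers fire OnDroppedToTerrain and a LifeTime-based takeoff, with empty functions as child hooks.
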(event Custom|EventForBackup)

(event EventBeginPlay
  (bind _returnvalue (Game|SpawnActorfromClass "/Game/GameElements/Objectives/Facility/Tethers/BP_HackingPod.BP_HackingPod_C" (Math|Transform|MakeTransform "0, 0,9999.000000") "AlwaysSpawn" 0 0))
  (bind _returnvalue_2 (Class|RessuplyPod|DroptoTarget _returnvalue "/Game/GameElements/Objectives/Facility/Tethers/BP_HackingPod.BP_HackingPod_C" (Class|FSDConversionLibrary|ActortoWorldLocation self)))
  (bind _asbp_hacking_pod (Utilities|Casting|CastToBP_HackingPod _returnvalue_2))
  (bind _output_get (Variables|Default|SetHackingPod _asbp_hacking_pod))
  (Utilities|FlowControl|Sequence
    (:then_0
      (Actor|DestroyActor _returnvalue)
      (Class|ActorComponent|SetIsReplicated (Variables|/Game/GameElements/Objectives/Facility/Tethers/BP_HackingPod.BP_HackingPod_C|GetBase _output_get) true)
      (Rendering|SetVisibility (Variables|/Game/GameElements/Objectives/Facility/Tethers/BP_HackingPod.BP_HackingPod_C|GetBase _output_get) false true)
      (Variables|Default|SetBaseComponent (Variables|/Game/GameElements/Objectives/Facility/Tethers/BP_HackingPod.BP_HackingPod_C|GetBase _output_get))
      (Actor|DestroyActor (Variables|/Script/Engine.ChildActorComponent|GetChildActor (Variables|/Game/GameElements/Objectives/Facility/Tethers/BP_HackingPod.BP_HackingPod_C|GetDispenserActor _output_get)))
      (Rendering|SetVisibility (Variables|/Game/GameElements/Objectives/Facility/Tethers/BP_HackingPod.BP_HackingPod_C|GetRangeSphere _output_get) false true)
      (Class|ActorComponent|SetIsReplicated (Variables|/Game/GameElements/Objectives/Facility/Tethers/BP_HackingPod.BP_HackingPod_C|GetWidget_MonitorLeft _output_get) true)
      (Rendering|SetVisibility (Variables|/Game/GameElements/Objectives/Facility/Tethers/BP_HackingPod.BP_HackingPod_C|GetWidget_MonitorLeft _output_get) false true)
      (Class|ActorComponent|SetIsReplicated (Variables|/Game/GameElements/Objectives/Facility/Tethers/BP_HackingPod.BP_HackingPod_C|GetWidget_MonitorRight _output_get) true)
      (Rendering|SetVisibility (Variables|/Game/GameElements/Objectives/Facility/Tethers/BP_HackingPod.BP_HackingPod_C|GetWidget_MonitorRight _output_get) false true)
      (Class|ActorComponent|SetIsReplicated (Variables|/Game/GameElements/Objectives/Facility/Tethers/BP_HackingPod.BP_HackingPod_C|GetWidget_MonitorMiddle _output_get) true)
      (Rendering|SetVisibility (Variables|/Game/GameElements/Objectives/Facility/Tethers/BP_HackingPod.BP_HackingPod_C|GetWidget_MonitorMiddle _output_get) false true)
      (Class|ActorComponent|SetIsReplicated (Variables|/Game/GameElements/Objectives/Facility/Tethers/BP_HackingPod.BP_HackingPod_C|GetWidget_MonitorTop _output_get) true)
      (Rendering|SetVisibility (Variables|/Game/GameElements/Objectives/Facility/Tethers/BP_HackingPod.BP_HackingPod_C|GetWidget_MonitorTop _output_get) false true)
      (Class|FacilityHackingPod|SetState _output_get "EClosed"))
    (:then_1
      (bind _actor (CallFunction|SpawnAlternateActor))
      (Transformation|AttachComponentToComponent _actor (Variables|Default|GetBaseComponent) "None" "KeepRelative" "KeepRelative" "KeepRelative" true)
      (bind _output_get_2 (Variables|Default|SetAlternateActor _actor))
      (CallFunction|AlternateActorSpawnedFunc _output_get_2)
      (Actor|SetLifeSpan _output_get_2 (+ (Variables|Default|GetLifeTime) 3e+01))
      (Utilities|FlowControl|Delay 15.0)
      (CallFunction|OnDroppedtoTerrain))
    (:then_2
      (Utilities|Time|SetTimerbyFunctionName 0 "TryTakeOff" (+ (Variables|Default|GetLifeTime) 15.0)))
    (:then_3
      (CallFunction|EventforBackup))))

(event Collision|EventActorBeginOverlap
  (params (OtherActor :type Actor%20Object%20Reference)))

(event EventTick
  (params (DeltaSeconds :type Float%20%28single-precision%29)))

(fn ConstructionScript)

(fn OnDroppedtoTerrain)

(fn SpawnAlternateActor
  (return 0))

(fn TryTakeOff
  (bind _hackingpod (Variables|Default|GetHackingPod))
  (if (not (Utilities|Enum|Equal(Enum) (Variables|/Script/FSD.FacilityHackingPod|GetPodState _hackingpod) "EDone"))
    (Class|FacilityHackingPod|SetState _hackingpod "EDone")
    (CallFunction|ExtraTakeOffFunc)))

(fn ExtraTakeOffFunc)

(fn AlternateActorSpawnedFunc
  (params (Actor :type Actor%20Object%20Reference)))