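; Engineer drop pod Blueprint that deploys an oversized BP_LureTarget, a holographic lure that enemies can attack.
; It fills in the parent pod's hooks, spawning the lure as the alternate actor with a long lifetime.
; After spawn it boosts the lure's health and hologram scale, tunes attacker positioning, and enables movement replication.
; The extra take-off hook plays the lure's Disappear timeline.
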(event Collision|EventActorBeginOverlap
  (params (OtherActor :type Actor%20Object%20Reference)))

(event EventTick
  (params (DeltaSeconds :type Float%20%28single-precision%29)))

(event EventBeginPlay
  (|CallParentFunction))

(fn ConstructionScript)

(fn OnDroppedtoTerrain)

(fn AlternateActorSpawnedFunc
  (params (Actor :type Actor%20Object%20Reference))
  (bind _asbp_lure_target (Utilities|Casting|CastToBP_LureTarget Actor))
  (bind _output_get (Variables|Default|SetLureTarget _asbp_lure_target))
  (Utilities|FlowControl|Sequence
    (:then_0
      (Variables|/Script/FSD.FriendlyHealthComponent|SetMaxHealth (Variables|/Game/WeaponsNTools/Grenades/Lure/BP_LureTarget.BP_LureTarget_C|GetFriendlyHealth _output_get) 1e+04)
      (Class|HealthComponentBase|Heal (Variables|/Game/WeaponsNTools/Grenades/Lure/BP_LureTarget.BP_LureTarget_C|GetFriendlyHealth _output_get) 1e+04)
      (Transformation|SetRelativeScale3D (Variables|/Game/WeaponsNTools/Grenades/Lure/BP_LureTarget.BP_LureTarget_C|GetMesh_Hologram _output_get) "1.300000,1.300000,1.300000"))
    (:then_1
      (Variables|/Script/FSD.AttackerPositioningComponent|SetCostModifier (Variables|/Game/WeaponsNTools/Grenades/Lure/BP_LureTarget.BP_LureTarget_C|GetObjectAttackerPositioning _output_get) 1.5)
      (Variables|/Script/FSD.AttackerPositioningComponent|SetMaxAttackers (Variables|/Game/WeaponsNTools/Grenades/Lure/BP_LureTarget.BP_LureTarget_C|GetObjectAttackerPositioning _output_get) 6)
      (Variables|/Script/FSD.AttackerPositioningComponent|SetCharacterHalfHeight (Variables|/Game/WeaponsNTools/Grenades/Lure/BP_LureTarget.BP_LureTarget_C|GetObjectAttackerPositioning _output_get) 45.0))
    (:then_2
      (Class|Actor|SetReplicateMovement _output_get true))))

(fn ExtraTakeOffFunc
  (Components|Timeline|PlayfromStart (Variables|/Game/WeaponsNTools/Grenades/Lure/BP_LureTarget.BP_LureTarget_C|GetDisappear (Variables|Default|GetLureTarget))))

(fn SpawnAlternateActor
  (bind _returnvalue (Game|SpawnActorfromClass "/Game/WeaponsNTools/Grenades/Lure/BP_LureTarget.BP_LureTarget_C" (Math|Transform|MakeTransform "0, 0, 0" "0, 0, 0" "1.300000,1.300000,1.300000") "AlwaysSpawn" 0 999.0 0))
  (return _returnvalue))