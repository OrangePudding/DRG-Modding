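; Applies the Burning Love random beer effect to a target player character, heating and periodically damaging them.
; On BeginPlay it adds the Burning Love and damage components to that character, then pushes a heat source for the effect's BeerEffectDurationSeconds.
; A looping half-second timer damages the character until the delay ends, pops the heat and sets TimeUp, which makes the timer clear itself.
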(event EventBeginPlay
  (bind _targetplayercharacter (Variables|Default|GetTargetPlayerCharacter))
  (Utilities|FlowControl|Sequence
    (:then_0
      (bind _returnvalue (AddComponent|AddDEBurningLove _targetplayercharacter))
      (bind _returnvalue_2 (AddComponent|AddDamageComponent _targetplayercharacter))
      (Variables|Default|SetDamage _returnvalue_2))
    (:then_1
      (Class|TemperatureComponent|TryPushHeatSource _targetplayercharacter 2e+02 "Cold1")
      (Utilities|FlowControl|Delay (Variables|/Script/FSD.DrinkEffectComponent|GetBeerEffectDurationSeconds _returnvalue))
      (Class|TemperatureComponent|TryPopHeatSource _targetplayercharacter 2e+02 "Cold1")
      (Variables|Default|SetTimeUp true))
    (:then_2
      (bind _returnvalue_3 (Utilities|Time|SetTimerbyFunctionName 0 "DoDamage" 0.5 true))
      (Variables|Default|SetDamageTimerHandle _returnvalue_3))))

(event Collision|EventActorBeginOverlap
  (params (OtherActor :type Actor%20Object%20Reference)))

(event EventTick
  (params (DeltaSeconds :type Float%20%28single-precision%29)))

(fn ConstructionScript)

(fn DoDamage
  (bind _targetplayercharacter (Variables|Default|GetTargetPlayerCharacter))
  (if (Variables|Default|GetTimeUp)
    (Utilities|Time|ClearandInvalidateTimerbyHandle (Variables|Default|GetDamageTimerHandle))
    (else
      (Class|DamageComponent|DamageTarget (Variables|Default|GetDamage) _targetplayercharacter (Class|FSDConversionLibrary|ActortoWorldLocation _targetplayercharacter)))))