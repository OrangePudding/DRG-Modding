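; Helper actor in a mod test folder that watches a Player's replicated perk usage and signals whenever a perk is used.
; BeginPlay snapshots each perk's used count from the controller's PerkUsageComponent into a map.
; Tick polls that array against the map, updating it and calling OnPerkUsed for new perks or changed counts.
; The actor destroys itself once the Player reference is invalid.
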(event EventBeginPlay
  (for _array_element (Variables|/Script/FSD.PerkUsageComponent|GetPerkUsageReplicated (Variables|/Script/FSD.FSDPlayerController|GetPerkUsageComponent (Class|PlayerCharacter|GetPlayerController (Variables|Default|GetPlayer))))
    (Utilities|Map|Add (Variables|Default|GetNewVar_0) (.Perk (Utilities|Struct|BreakPerkUsage _array_element)) (.UsedCount (Utilities|Struct|BreakPerkUsage _array_element)))))

(event Collision|EventActorBeginOverlap
  (params (OtherActor :type Actor%20Object%20Reference)))

(event EventTick
  (params (DeltaSeconds :type Float%20%28single-precision%29))
  (if (Utilities|IsValid (Variables|Default|GetPlayer))
    (CallFunction|CheckPerkUsage)
    (else
      (Actor|DestroyActor))))

(fn ConstructionScript)

(fn CheckPerkUsage
  (bind _newvar_0 (Variables|Default|GetNewVar_0))
  (for _array_element (Variables|/Script/FSD.PerkUsageComponent|GetPerkUsageReplicated (Variables|/Script/FSD.FSDPlayerController|GetPerkUsageComponent (Class|PlayerCharacter|GetPlayerController (Variables|Default|GetPlayer))))
    (if (.ReturnValue (Utilities|Map|Find _newvar_0 (.Perk (Utilities|Struct|BreakPerkUsage _array_element))))
      (if (!= (.Value (Utilities|Map|Find _newvar_0 (.Perk (Utilities|Struct|BreakPerkUsage _array_element)))) (.UsedCount (Utilities|Struct|BreakPerkUsage _array_element)))
        (Utilities|Map|Add _newvar_0 (.Perk (Utilities|Struct|BreakPerkUsage _array_element)) (.UsedCount (Utilities|Struct|BreakPerkUsage _array_element)) :!label _label)
        (Default|CallOnPerkUsed (.Perk (Utilities|Struct|BreakPerkUsage _array_element))))
      (else
        (goto _label)))))