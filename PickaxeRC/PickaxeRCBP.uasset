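; PickaxeRCBP changes the local player's first-person pickaxe animations in what appears to be a Deep Rock Galactic mod.
; BeginPlay polls for the character and controller, then listens for equipped items to cache the pickaxe and bind its target-damaged event.
; Each hit sets the equip animation to an attack montage and plays it on FPMesh, posting debug messages.
; Equipping a non-pickaxe item restores the cached pickaxe's normal equip animation.
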(event Custom|OnItemEquipped_Event_0
  (params (Item :type Item%20Object%20Reference))
  ;[1 1 1] On Equipped
  (bind _aswpn_pickaxe (Utilities|Casting|CastToWPN_Pickaxe Item)
    (:then
      (if (!= _aswpn_pickaxe (Variables|Default|GetAs%20WPN%20Pickaxe))
        (bind _output_get (Variables|Default|SetAs%20WPN%20Pickaxe _aswpn_pickaxe))
        (EventDispatchers|BindEventtoOnTargetDamagedEvent (Variables|/Script/FSD.PickaxeItem|GetDamageComponent _output_get) (delegate Custom|OnTargetDamagedEvent_Event_0))))
    (:CastFailed
      (if (!= 0 (Variables|Default|GetAs%20WPN%20Pickaxe))
        (Variables|/Script/FSD.PickaxeItem|SetFP_EquipAnimation (Variables|Default|GetAs%20WPN%20Pickaxe) "/Game/CharacterStructure/Gear_Pickaxe/FP/FP_Pickaxe_Equip_Montage.FP_Pickaxe_Equip_Montage")))))

(event Custom|OnTargetDamagedEvent_Event_0
  (params (Health :type Health%20Component%20Base%20Object%20Reference) (amount :type Float%20%28single-precision%29) (Component :type Primitive%20Component%20Object%20Reference) (PhysicalMaterial :type FSD%20Physical%20Material%20Object%20Reference))
  (bind _returnvalue (Class|GameFunctionLibrary|GetFSDGameState))
  ;[1 1 1] On Equipped
  (Variables|/Script/FSD.PickaxeItem|SetFP_EquipAnimation (Variables|Default|GetAs%20WPN%20Pickaxe) "/Game/PickaxeRC/Anims/FP/FP_BXE_Pickaxe_Attack_A_Montage.FP_BXE_Pickaxe_Attack_A_Montage")
  (Animation|Montage|PlayMontage (Variables|/Script/FSD.PlayerCharacter|GetFPMesh (Class|GameFunctionLibrary|GetLocalPlayerCharacter)) "/Game/PickaxeRC/Anims/FP/FP_BXE_Pickaxe_Attack_A_Montage.FP_BXE_Pickaxe_Attack_A_Montage" 1.0 0.0 "Default"
    (:then
      (Class|FSDGameState|PostGameMessage _returnvalue "Triggered"))
    (:OnCompleted
      (Class|FSDGameState|PostGameMessage _returnvalue "Completed"))
    (:OnInterrupted
      (Class|FSDGameState|PostGameMessage _returnvalue "Interrupted"))))

(event EventBeginPlay
  (bind _returnvalue (Class|GameFunctionLibrary|GetLocalPlayerCharacter))
  ;[1 1 1] Startup Stuff
  (Utilities|IsValid _returnvalue :!label _label
    (:Is%20Valid
      (Utilities|IsValid (Class|PlayerCharacter|GetPlayerController _returnvalue) :!label _label_2
        (:Is%20Valid
          ;[1 1 1] On Equipped
          (EventDispatchers|AssignOnItemEquipped (Variables|/Script/FSD.PlayerCharacter|GetInventoryComponent (Class|GameFunctionLibrary|GetLocalPlayerCharacter)) (delegate Custom|OnItemEquipped_Event_0)))
        (:Is%20Not%20Valid
          (Utilities|FlowControl|Delay 0.2)
          (goto _label_2))))
    (:Is%20Not%20Valid
      (Utilities|FlowControl|Delay 0.2)
      (goto _label))))

(fn ConstructionScript)