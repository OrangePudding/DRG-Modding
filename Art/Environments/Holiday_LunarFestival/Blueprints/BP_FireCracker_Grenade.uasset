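; BP_FireCracker_Grenade is a Lunar Festival firecracker grenade that explodes after a fuse delay.
; BeginPlay starts a timer that calls DetonateFireCracker by function name once FuseTime elapses.
; Detonation calls DamageAndCarve on the Explosion component at the actor's location, passing the default physical material and the Damage component to deal damage and carve.
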(event EventBeginPlay
  (|CallParentFunction)
  (Utilities|Time|SetTimerbyFunctionName 0 "DetonateFireCracker" (Variables|Default|GetFuseTime)))

(event Collision|EventActorBeginOverlap
  (params (OtherActor :type Actor%20Object%20Reference))
  (|CallParentFunction OtherActor) ; This node is disabled and will not be called.\nDrag off pins to build functionality.
)

(event EventTick
  (params (DeltaSeconds :type Float%20%28single-precision%29))
  (|CallParentFunction DeltaSeconds) ; This node is disabled and will not be called.\nDrag off pins to build functionality.
)

(fn ConstructionScript
  (|CallParentFunction))

(fn DetonateFireCracker
  (Class|ExplosionBaseComponent|DamageandCarve (Variables|Default|GetExplosion) (Transformation|GetActorLocation) "0, 0, 0" "None" 0 "/Engine/EngineMaterials/DefaultPhysicalMaterial.DefaultPhysicalMaterial" (Variables|Default|GetDamage)))