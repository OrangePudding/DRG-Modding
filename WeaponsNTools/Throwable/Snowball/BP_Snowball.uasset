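; BP_Snowball is a short-lived throwable snowball actor that replaces itself with a PRJ_Crye_SnowBall ballistic projectile on BeginPlay.
; It spawns a temporary projectile solely to call SpawnBallisticProjectile, passing its own location, velocity and instigator.
; The resulting projectile gets its radial damage scaled by RadialDamageMultiplier and is shrunk to half size.
; The temporary projectile and this actor then destroy themselves.
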(event EventBeginPlay
  (bind _self self)
  (bind _returnvalue (Game|GetInstigator _self))
  (bind _returnvalue_2 (Game|SpawnActorfromClass "/Game/WeaponsNTools/Cryospray/PRJ_Crye_SnowBall.PRJ_Crye_SnowBall_C" (Transformation|GetActorTransform _self) "AlwaysSpawn" (Components|GetOwner _self) _returnvalue))
  (bind _returnvalue_3 (Class|Projectile|SpawnBallisticProjectile _returnvalue_2 "/Game/WeaponsNTools/Cryospray/PRJ_Crye_SnowBall.PRJ_Crye_SnowBall_C" _returnvalue (Class|FSDConversionLibrary|ActortoWorldLocation _self) (Transformation|GetVelocity _self)))
  (bind _asprj_crye_snow_ball (Utilities|Casting|CastToPRJ_Crye_SnowBall _returnvalue_3))
  (Variables|/Script/FSD.DamageComponent|SetRadialDamage (Variables|/Game/WeaponsNTools/Cryospray/PRJ_Crye_SnowBall.PRJ_Crye_SnowBall_C|GetDamage _asprj_crye_snow_ball) (* (Variables|/Script/FSD.DamageComponent|GetRadialDamage (Variables|/Game/WeaponsNTools/Cryospray/PRJ_Crye_SnowBall.PRJ_Crye_SnowBall_C|GetDamage _asprj_crye_snow_ball)) (Variables|Default|GetRadialDamageMultiplier)))
  (Transformation|SetActorScale3D _asprj_crye_snow_ball "0.500000,0.500000,0.500000")
  (Actor|DestroyActor _returnvalue_2)
  (Actor|DestroyActor))

(event Collision|EventActorBeginOverlap
  (params (OtherActor :type Actor%20Object%20Reference)))

(event EventTick
  (params (DeltaSeconds :type Float%20%28single-precision%29)))

(fn ConstructionScript)